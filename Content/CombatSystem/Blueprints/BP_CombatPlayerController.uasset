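; Player controller for the combat system that creates the main HUD and wires its inventory, equipment, attribute and level widgets to the possessed character's inventory and stats components.
; Toggling the inventory freezes movement, switches the character camera and plays a sound.
; Two counters manage nested UI: one controls cursor and input mode, the other blocks toggling while child widgets are open.
; It also relays potion counts and exposes HUD and options-menu references.
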(event `self.ReceiveBeginPlay`
  (bind _mainhud (`self.MainHUD`))
  (bind _returnvalue (`self.GetComponentByClass` (`self.CharacterRef`) "/Game/CombatSystem/Blueprints/Components/BP_StatsComponent.BP_StatsComponent_C"))
  (bind _returnvalue_2 (`self.GetComponentByClass` (`self.CharacterRef`) "/Game/CombatSystem/Blueprints/Components/BP_InventoryComponent.BP_InventoryComponent_C"))
  (bind _wb_inventory (`/Game/CombatSystem/UI/WBP_MainHUD.WB_Inventory` (`self.MainHUD`)))
  (bind _wb_inventory_2 (`/Game/CombatSystem/UI/WBP_MainHUD.WB_Inventory` _mainhud))
  (bind _returnvalue_3 (`|CreateWidget` "/Game/CombatSystem/UI/WBP_MainHUD.WBP_MainHUD_C" self))
  (bind _output_get (set `self.MainHUD` _returnvalue_3))
  (`UserWidget.AddToViewport` _output_get 0)
  (set `/Game/CombatSystem/UI/WB_Inventory.WBP_MainHUDRef` _mainhud _wb_inventory_2)
  (`/Game/CombatSystem/UI/WB_InventoryWindow.Setup` (`/Game/CombatSystem/UI/WB_Inventory.WB_InventoryWindow` _wb_inventory_2) _returnvalue_2)
  (set `/Game/CombatSystem/UI/WB_Equipment.InventoryComponent` _returnvalue_2 (`/Game/CombatSystem/UI/WB_Inventory.WB_Equipment` _wb_inventory))
  (`/Game/CombatSystem/UI/WB_CharacterAttributes.Setup` (`/Game/CombatSystem/UI/WB_Inventory.WB_CharacterAttributes` _wb_inventory) _returnvalue)
  (`/Game/CombatSystem/UI/WB_LevelTracker.SetupLink` (`/Game/CombatSystem/UI/WB_Inventory.WB_LevelTracker` (`/Game/CombatSystem/UI/WBP_MainHUD.WB_Inventory` (`self.MainHUD`))) _returnvalue))

(event `self.ReceivePossess`
  (params (PossessedPawn :type "Pawn Object Reference"))
  (bind _ascharacter (cast `Character` PossessedPawn))
  (set `self.CharacterRef` _ascharacter))

(event `SetPotionAmount`
  (params (Amount :type Integer))
  (bind _mainhud (`self.MainHUD`)
    (:`then`
      (`/Game/CombatSystem/UI/WBP_MainHUD.SetPotionAmount` _mainhud Amount))
    (:`else`)))

(event `/Game/CombatSystem/Blueprints/Interfaces/PlayerController_BPI.ToggleInventory`
  (bind _inventoryopen (`self.InventoryOpen`))
  (bind _wb_inventory (`/Game/CombatSystem/UI/WBP_MainHUD.WB_Inventory` (`self.MainHUD`)))
  (if (`self.CanToggleWIdget`)
    (if (not (`/Game/CombatSystem/UI/WB_Inventory.MidAnimation` _wb_inventory))
      (set `self.InventoryOpen` (not (`self.InventoryOpen`)))
      (`CharacterMovementComponent.SetMovementMode` (`Character.CharacterMovement` (`self.CharacterRef`)) (select `bool` _inventoryopen :`false` "MOVE_Walking" :`true` "MOVE_None" :!type "EMovementMode Enum") 0)
      (message `/Game/CombatSystem/Blueprints/Interfaces/Character_BPI.ToggleInventoryCamera` (`self.CharacterRef`) _inventoryopen)
      (`self.SetUICounter` _inventoryopen)
      (`/Game/CombatSystem/UI/WB_Inventory.ToggleInventory` _wb_inventory (select `bool` _inventoryopen :`false` "NewEnumerator1" :`true` "NewEnumerator0" :!type "/Game/CombatSystem/Blueprints/Enums/E_InventoryStatusWB Enum"))
      (`GameplayStatics.PlaySound2D` "/Game/CombatSystem/CourseFiles/SoundFX/UI/SW_OpenSpellbook_02.SW_OpenSpellbook_02" 1.0 1.0 0.0 null null))))

(event `/Game/CombatSystem/Blueprints/Interfaces/PlayerController_BPI.ReceiveOptionsMenu`
  (params (OptionsMenu :type "/Game/CombatSystem/UI/WB_OptionList Object Reference"))
  (set `self.WBOptionsMenu` OptionsMenu))

(fn `InventoryStatus`
  (returns (InventoryOpen :type Boolean))
  (return (`self.InventoryOpen`)))

(fn `IsWidgetsOpen?`
  (returns (ReturnValue :type Boolean))
  (return (`self.InventoryOpen`)))

(fn `PassHUDWB`
  (returns (MainHUD :type "/Game/CombatSystem/UI/WBP_MainHUD Object Reference"))
  (return (`self.MainHUD`)))

(fn `PassOptionsMenu`
  (returns (OptionsMenu :type "/Game/CombatSystem/UI/WB_OptionList Object Reference"))
  (return (`self.WBOptionsMenu`)))

(fn `SetCanUpdateWidget`
  (params (CanUpdateWidget :type Boolean))
  (bind _counter (`self.Counter`))
  ;[0.4442 0.9273 1] Prevents Widgets From Opening Closing - Needed for when a widget has created a widget, don't want to close first widget until second widget is removed. E.g. Inventory Open, Drop Item widget created = Prevent Inventory Closing until drop item widget closed
  (if CanUpdateWidget
    (`/Engine/EditorBlueprintResources/StandardMacros.DecrementInt` _counter
      (:`  `
        _))
    (else
      (`/Engine/EditorBlueprintResources/StandardMacros.IncrementInt` _counter
        (:`  `
          _))))
  (set `self.CanToggleWIdget` (== _counter 0))
  (return))

(fn `SetUICounter`
  (params (SetVisible :type Boolean))
  (if SetVisible
    ;[0.7022 1 0.7104] Increase UI Counter - Show Mouse Cursor - Input Mode Game And UI
    (`/Engine/EditorBlueprintResources/StandardMacros.IncrementInt` (`self.UI_Open`)
      (:`  `
        (if (not (`self.bShowMouseCursor`))
          (`WidgetBlueprintLibrary.SetInputMode_GameAndUIEx` self null)
          (set `self.bShowMouseCursor` true))))
    (else
      ;[1 0.6295 0.6928] Decrament UI Counter - Hide Mouse Cursor - Input Mode Game Only
      (bind _result (`/Engine/EditorBlueprintResources/StandardMacros.DecrementInt` (`self.UI_Open`))
        (:`  `
          (if (== _result 0)
            (`WidgetBlueprintLibrary.SetInputMode_GameOnly` self)
            (set `self.bShowMouseCursor` false)))))))

(fn `UserConstructionScript`)