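; Combat hit-detection component that sweeps a weapon or other mesh for hits while collision is active.
; Each tick it runs a multi-sphere object trace between start and end sockets on the assigned mesh, excluding ignored actors.
; Hits pass a gameplay-tag filter and a once-per-activation check before firing the OnHit callback.
; Activating collision clears the already-hit list; deactivating stops tracing.
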(event `self.ReceiveTick`
  (params (DeltaSeconds :type "Float (single-precision)"))
  (if (`self.bIsCollisionEnabled?`)
    (`self.CollisionTrace`)))

(event `SetCollisionMesh`
  (params (CollisionMeshComponent :type "PrimitiveComponent Object Reference"))
  ;[1 0 0] Set CollisionMesh Component
  (set `self.CollisionMeshComponent` CollisionMeshComponent))

(event `CollisionTrace`
  (bind _collisionmeshcomponent (`self.CollisionMeshComponent`))
  ;[1 0 0] Collision Trace
  (bind _outhits (`KismetSystemLibrary.SphereTraceMultiForObjects` (`SceneComponent.GetSocketLocation` _collisionmeshcomponent (`self.StartSocketName`)) (`SceneComponent.GetSocketLocation` _collisionmeshcomponent (`self.EndSocketName`)) (`self.TraceRadius`) (`self.CollisionObjectTypes`) false (`self.ActorsToIgnore`) (`self.Draw Debug Type`) true (struct :`R` 1.0 :`A` 1.0) (struct :`G` 1.0 :`A` 1.0) 2.0))
  (for _array_element _outhits
    (bind _output_get (set `self.LastHit` _array_element))
    (bind (_bblockinghit _binitialoverlap _time _distance _location _impactpoint _normal _impactnormal _physmat _hitactor) (`GameplayStatics.BreakHitResult` _output_get))
    (if (`self.Can Hit Actor?` _hitactor)
      (bind _output_get_2 (set `self.Hit Actor` _hitactor))
      (`KismetArrayLibrary.Array_AddUnique` (`self.AlreadyHitActors`) _output_get_2)
      (`self.OnHit` (`self.LastHit`)))))

(event `ActivateCollision`
  ;[1 0 0] Activate Collision
  (`self.ClearHitActors`)
  (set `self.bIsCollisionEnabled?` true))

(event `DeactivateCollision`
  ;[1 0 0] Deactivate Collision
  (set `self.bIsCollisionEnabled?` false))

(event `ClearHitActors`
  ;[1 0 0] Clear Hit Actors
  (`KismetArrayLibrary.Array_Clear` (`self.AlreadyHitActors`)))

(fn `AddActorToIgnore`
  (params (InActor :type "Actor Object Reference (by ref)"))
  (`KismetArrayLibrary.Array_AddUnique` (`self.ActorsToIgnore`) InActor))

(fn `Can Hit Actor?`
  (params (InActor :type "Actor Object Reference (by ref)"))
  (returns (ReturnValue :type Boolean))
  (bind _returnvalue (message `/Game/CombatSystem/Blueprints/Interfaces/GameplayTagBlueprintInterface.GetOwnedGameplayTags` InActor))
  (return (and (not (`BlueprintGameplayTagLibrary.HasAnyTags` _returnvalue (`self.GameplayTagsToIgnore`))) (not (`KismetArrayLibrary.Array_Contains` (`self.AlreadyHitActors`) InActor)))))

(fn `GetActorToIgnore`
  (returns (ActorsToIgnore :type "Array of Actor Object Reference"))
  (return (`self.ActorsToIgnore`)))

(fn `GetAlreadyHitActors`
  (returns (ReturnValue :type "Array of Actor Object Reference"))
  (return (`self.AlreadyHitActors`)))

(fn `GetCollisionMeshComponent`
  (returns (ReturnValue :type "PrimitiveComponent Object Reference"))
  (return (`self.CollisionMeshComponent`)))

(fn `GetLastHit`
  (returns (ReturnValue :type "HitResult Structure"))
  (return (`self.LastHit`)))

(fn `IsCollisionEnabled?`
  (returns (ReturnValue :type Boolean))
  (return (`self.bIsCollisionEnabled?`)))

(fn `RemoveActorToIgnore`
  (params (ActorToRemove :type "Actor Object Reference (by ref)"))
  (`KismetArrayLibrary.Array_RemoveItem` (`self.ActorsToIgnore`) ActorToRemove))