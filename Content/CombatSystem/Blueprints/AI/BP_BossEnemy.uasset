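; BP_BossEnemy is a boss AI character that extends a parent enemy with a melee weapon and an on-screen health bar.
; The health widget binds to the stats component, appears when the boss has a valid target and hides on target loss or death.
; Weapon collision hits apply stat-based point damage to damageable actors.
; The weapon switches sockets as combat toggles and simulates physics on death.
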(event `self.ReceiveBeginPlay`
  (`parent.ReceiveBeginPlay`)
  (`/Game/CombatSystem/Blueprints/Components/BP_CollisionComponent.SetCollisionMesh` (`self.MainWeaponCollisionComponent`) (`self.WeaponMesh`))
  (bind _returnvalue (`|CreateWidget` "/Game/CombatSystem/UI/WBP_BossHealth.WBP_BossHealth_C" (`GameplayStatics.GetPlayerController` 0)))
  (bind _output_get (set `self.BossHealthUI` _returnvalue))
  (`/Game/CombatSystem/UI/WBP_BossHealth.Initialize` _output_get (`self.StatsComponent`))
  (`UserWidget.AddToViewport` _output_get 0))

(event `/Game/CombatSystem/Blueprints/Interfaces/Targeting_BPI.OnTargeted`
  (params (`bIsTargeted?` :type Boolean))
  (`parent.OnTargeted` `bIsTargeted?`))

(event `SetBossHealthVisibility`
  (params (`bVisible?` :type Boolean))
  (bind _bosshealthui (`self.BossHealthUI`)
    (:`then`
      (`Widget.SetVisibility` _bosshealthui (select `bool` (and `bVisible?` (not (`/Game/CombatSystem/Blueprints/Components/BP_StateManagerComponent.IsCurrentStateEqualToAny?` (`self.StateManagerComponent`) (struct :`GameplayTags` (struct :`(TagName` "Character.State.Dead")))))) :`false` "Hidden" :`true` "Visible" :!type "ESlateVisibility Enum")))
    (:`else`)))

(event `self.MainWeaponCollisionComponent.OnHit`
  (params (HitResult :type "HitResult Structure"))
  (bind (_bblockinghit _binitialoverlap _time _distance _location _impactpoint _normal _impactnormal _physmat _hitactor) (`GameplayStatics.BreakHitResult` HitResult))
  (bind _returnvalue (message `/Game/CombatSystem/Blueprints/Interfaces/Combat_BPI.CanReceiveDamage` _hitactor))
  (if _returnvalue
    (`GameplayStatics.ApplyPointDamage` _hitactor (`/Game/CombatSystem/Blueprints/Components/BP_StatsComponent.GetCurrentStatValue` (`self.StatsComponent`) "NewEnumerator4") (`self.GetActorForwardVector`) HitResult (`self.GetController`) self (`self.Damage Type Class`))))

(event `SimulateWeaponPhysics`
  (`PrimitiveComponent.SetCollisionProfileName` (`self.WeaponMesh`) "PhysicsActor" true)
  (`PrimitiveComponent.SetSimulatePhysics` (`self.WeaponMesh`) true))

(event `self.CombatComponent.OnCombatToggled`
  (params (`bIsCombatEnabled?` :type Boolean))
  (`SceneComponent.K2_AttachToComponent` (`self.WeaponMesh`) (`self.Mesh`) (select `bool` `bIsCombatEnabled?` :`false` (`self.AttachSocketName`) :`true` (`self.WeaponHandSocket`)) "SnapToTarget" "SnapToTarget" "SnapToTarget" true))

(event `self.PerformDeath`
  (`parent.PerformDeath`)
  (`self.SimulateWeaponPhysics`)
  (`self.SetBossHealthVisibility` false))

(event `self.OnTargetSet`
  (params (NewTarget :type "Actor Object Reference"))
  (`parent.OnTargetSet` NewTarget)
  (`self.SetBossHealthVisibility` (`KismetSystemLibrary.IsValid` NewTarget)))

(fn `UserConstructionScript`
  (`parent.UserConstructionScript`))