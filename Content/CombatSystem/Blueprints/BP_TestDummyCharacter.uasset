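; BP_TestDummyCharacter is a target dummy character for testing the combat system.
; It initializes its StatsComponent on BeginPlay and shows or hides its lock-on widget as it gains or loses targeting.
; It can be targeted unless its StateManagerComponent reports the Dead state, and it always returns one fixed movement speed mode.
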(event `self.ReceiveBeginPlay`
  (`/Game/CombatSystem/Blueprints/Components/BP_StatsComponent.InitializeStats` (`self.StatsComponent`)))

(event `/Game/CombatSystem/Blueprints/Interfaces/Targeting_BPI.OnTargeted`
  (params (`bIsTargeted?` :type Boolean))
  (`SceneComponent.SetVisibility` (`self.LockOnWidget`) `bIsTargeted?` false))

(fn `CanBeTargeted?`
  (returns (ReturnValue :type Boolean))
  (return (not (`/Game/CombatSystem/Blueprints/Components/BP_StateManagerComponent.IsCurrentStateEqualToAny?` (`self.StateManagerComponent`) (struct :`GameplayTags` (struct :`(TagName` "Character.State.Dead")))))))

(fn `GetMovementSpeedMode`
  (returns (MovementSpeedMode :type "/Game/CombatSystem/Blueprints/Enums/E_MovementSpeedMode Enum"))
  (return "NewEnumerator0"))

(fn `UserConstructionScript`
  (`parent.UserConstructionScript`))