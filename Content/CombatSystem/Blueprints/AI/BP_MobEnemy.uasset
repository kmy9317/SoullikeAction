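; BP_MobEnemy is an enemy character Blueprint that extends its parent with weapon combat, a health bar and a hearing indicator.
; On BeginPlay it sets up weapon collision and creates both widgets, showing the health bar when targeting changes and toggling the hearing icon on request.
; Weapon hits apply stat-based point damage to valid actors.
; Combat toggling moves the weapon between hand and attach sockets, and death makes it simulate physics.
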(event `self.ReceiveBeginPlay`
  (`parent.ReceiveBeginPlay`)
  (`/Game/CombatSystem/Blueprints/Components/BP_CollisionComponent.SetCollisionMesh` (`self.MainWeaponCollisionComponent`) (`self.GetWeaponMesh`))
  (bind _returnvalue (`|CreateWidget` "/Game/CombatSystem/UI/WBP_HealthBar.WBP_HealthBar_C" (`GameplayStatics.GetPlayerController` 0) (`self.StatsComponent`) false))
  (`WidgetComponent.SetWidget` (`self.HealthBar`) _returnvalue)
  (bind _returnvalue_2 (`|CreateWidget` "/Game/CombatSystem/UI/WB_Hearing.WB_Hearing_C" (`GameplayStatics.GetPlayerController` 0) self))
  (set `self.HearingWidget` _returnvalue_2)
  (`WidgetComponent.SetWidget` (`self.HearingIcon`) _returnvalue_2))

(event `/Game/CombatSystem/Blueprints/Interfaces/Targeting_BPI.OnTargeted`
  (params (`bIsTargeted?` :type Boolean))
  (`parent.OnTargeted` `bIsTargeted?`)
  (`SceneComponent.SetVisibility` (`self.HealthBar`) `bIsTargeted?` false))

(event `self.MainWeaponCollisionComponent.OnHit`
  (params (HitResult :type "HitResult Structure"))
  (bind (_bblockinghit _binitialoverlap _time _distance _location _impactpoint _normal _impactnormal _physmat _hitactor) (`GameplayStatics.BreakHitResult` HitResult))
  (bind _returnvalue (message `/Game/CombatSystem/Blueprints/Interfaces/Combat_BPI.CanReceiveDamage` _hitactor))
  (if _returnvalue
    (`GameplayStatics.ApplyPointDamage` _hitactor (`/Game/CombatSystem/Blueprints/Components/BP_StatsComponent.GetCurrentStatValue` (`self.StatsComponent`) "NewEnumerator4") (`self.GetActorForwardVector`) HitResult (`self.GetController`) self (`self.Damage Type Class`))))

(event `SimulateWeaponPhysics`
  (bind _returnvalue (`self.GetWeaponMesh`))
  (`PrimitiveComponent.SetCollisionProfileName` _returnvalue "PhysicsActor" true)
  (`PrimitiveComponent.SetSimulatePhysics` _returnvalue true))

(event `self.CombatComponent.OnCombatToggled`
  (params (`bIsCombatEnabled?` :type Boolean))
  (`SceneComponent.K2_AttachToComponent` (`self.GetWeaponMesh`) (`self.Mesh`) (select `bool` `bIsCombatEnabled?` :`false` (`self.AttachSocketName`) :`true` (`self.WeaponHandSocket`)) "SnapToTarget" "SnapToTarget" "SnapToTarget" true))

(event `self.PerformDeath`
  (`parent.PerformDeath`)
  (`self.SimulateWeaponPhysics`))

(event `/Game/CombatSystem/Blueprints/Interfaces/Enemy_BPI.HearingVisibility`
  (params (Visibility :type Boolean))
  (`Widget.SetVisibility` (`/Game/CombatSystem/UI/WB_Hearing.EyeIcon` (`self.HearingWidget`)) (select `bool` Visibility :`false` "Hidden" :`true` "Visible" :!type "ESlateVisibility Enum")))

(fn `UserConstructionScript`
  (`parent.UserConstructionScript`))