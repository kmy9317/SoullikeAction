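; Character component that manages walking, jogging, sprinting and crouching for its owner.
; Each mode change notifies the targeting component to update rotation, then a looping timer interpolates max walk and crouched speed toward the mode's target.
; Sprinting requires a moving, grounded, uncrouched character and starts a repeating timer for draining stamina through the stats component.
; Crouch toggling also calls the character's crouch functions and broadcasts the change.
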(event `self.ReceiveBeginPlay`
  ;[1 0 0] Initialize
  (`self.Initialize`))

(event `AdjustMovementSpeed`
  ;[1 0 0] Adjust movement speed
  (set `self.WalkSpeedTarget` (select `/Game/CombatSystem/Blueprints/Enums/E_MovementSpeedMode` (`self.MovementSpeedMode`) :`NewEnumerator0` 200.0 :`NewEnumerator1` (`self.DefaultMaxWalkSpeed`) :`NewEnumerator2` 700.0 :`NewEnumerator5` 250.0))
  (set `self.MovementSpeedRef` (`CharacterMovementComponent.MaxWalkSpeed` (`self.Character Movement`)))
  (bind _returnvalue (`KismetSystemLibrary.K2_SetTimerDelegate` (delegate `LerpMovement`) 0.01 true)))

(event `LerpMovement`
  (bind _character_movement (`self.Character Movement`))
  ;[1 0 0] Adjust movement speed
  (bind _output_get (set `CharacterMovementComponent.MaxWalkSpeed` (`KismetMathLibrary.FInterpTo` (`CharacterMovementComponent.MaxWalkSpeed` (`self.Character Movement`)) (`self.WalkSpeedTarget`) (`GameplayStatics.GetWorldDeltaSeconds`) 10.0) _character_movement))
  (set `CharacterMovementComponent.MaxWalkSpeedCrouched` _output_get _character_movement)
  (if (`KismetMathLibrary.NearlyEqual_FloatFloat` (`CharacterMovementComponent.MaxWalkSpeed` (`self.Character Movement`)) (`self.WalkSpeedTarget`) 1.0)
    (`KismetSystemLibrary.K2_ClearAndInvalidateTimerHandle` (stale `AdjustMovementSpeed` _returnvalue))))

(event `Event Sprint`
  ;[1 0 0] Sprint
  (if (`self.CanPerformSprint`)
    (`self.SetMovementSpeedMode` "NewEnumerator2")
    (`self.AdjustMovementSpeed`)
    (bind _returnvalue (`KismetSystemLibrary.K2_SetTimerDelegate` (`|CreateDelegate` :!event `DrainSprintStaminaCost`) 0.1 true))
    (set `self.DrainStaminaTimer` _returnvalue)))

(event `DrainSprintStaminaCost`
  ;[1 0 0] Sprint
  (if (`self.CanPerformSprint`)
    (`/Game/CombatSystem/Blueprints/Components/BP_StatsComponent.ModifyCurrentStatValue` (`self.StatsComponent`) "NewEnumerator2" (`self.StaminaDrained`) true)
    (if (< (`/Game/CombatSystem/Blueprints/Components/BP_StatsComponent.GetCurrentStatValue` (`self.StatsComponent`) "NewEnumerator2") 10.0)
      (`self.Event ReleaseSprint`))
    (else
      (`self.Event ReleaseSprint`))))

(event `Event ReleaseSprint`
  ;[1 0 0] Sprint
  (`KismetSystemLibrary.K2_ClearAndInvalidateTimerHandle` (`self.DrainStaminaTimer`))
  (if (`|EnumEquality` (`self.MovementSpeedMode`) "NewEnumerator2")
    (`self.SetMovementSpeedMode` "NewEnumerator1")
    (`self.AdjustMovementSpeed`)))

(event `Event ToggleWalking`
  ;[1 0 0] Walking and jogging
  (if (`self.CanPeformToggleWalking`)
    (if (`|EnumInequality` (`self.MovementSpeedMode`) "NewEnumerator0")
      (`self.SetMovementSpeedMode` "NewEnumerator0")
      (`self.AdjustMovementSpeed`)
      (else
        (`self.SetMovementSpeedMode` "NewEnumerator1")
        (`self.AdjustMovementSpeed`)))))

(event `Event ToggleCrouch`
  ;[1 0 0] Crouch
  (if (`|EnumInequality` (`self.MovementSpeedMode`) "NewEnumerator5")
    (`self.SetMovementSpeedMode` "NewEnumerator5")
    (`self.AdjustMovementSpeed`)
    (`Character.Crouch` (`self.Character`))
    (`self.OnCrouch` true)
    (else
      (`self.SetMovementSpeedMode` "NewEnumerator1")
      (`self.AdjustMovementSpeed`)
      (`Character.UnCrouch` (`self.Character`))
      (`self.OnCrouch` false))))

(fn `CanPeformToggleWalking`
  (returns (ReturnValue :type Boolean))
  (bind _character_movement (`self.Character Movement`))
  (return (and (not (`NavMovementComponent.IsCrouching` _character_movement)) (not (`NavMovementComponent.IsFalling` _character_movement)))))

(fn `CanPerformSprint`
  (returns (ReturnValue :type Boolean))
  (bind _character_movement (`self.Character Movement`))
  (return (and (!= (`KismetMathLibrary.VSize` (`Actor.GetVelocity` (`self.Character`))) 0.0) (not (`NavMovementComponent.IsCrouching` _character_movement)) (not (`NavMovementComponent.IsFalling` _character_movement)))))

(fn `GetCurrentSpeedMode`
  (returns (MovementSpeedMode :type "/Game/CombatSystem/Blueprints/Enums/E_MovementSpeedMode Enum"))
  (return (`self.MovementSpeedMode`)))

(fn `Initialize`
  (bind _returnvalue (`self.GetOwner`))
  (set `self.StatsComponent` (`Actor.GetComponentByClass` _returnvalue "/Game/CombatSystem/Blueprints/Components/BP_StatsComponent.BP_StatsComponent_C"))
  (set `self.CombatComponent` (`Actor.GetComponentByClass` _returnvalue "/Game/CombatSystem/Blueprints/Components/BP_CombatComponent.BP_CombatComponent_C"))
  (set `self.StateManagerComponent` (`Actor.GetComponentByClass` _returnvalue "/Game/CombatSystem/Blueprints/Components/BP_StateManagerComponent.BP_StateManagerComponent_C"))
  (set `self.TargetingComponent` (`Actor.GetComponentByClass` _returnvalue "/Game/CombatSystem/Blueprints/Components/BP_TargetingComponent.BP_TargetingComponent_C"))
  (bind _ascharacter (cast `Character` _returnvalue))
  (set `self.Mesh` (`Character.Mesh` _ascharacter))
  (bind _charactermovement (`Character.CharacterMovement` _ascharacter))
  (set `self.Character Movement` _charactermovement)
  (set `self.Character` _ascharacter)
  (set `self.DefaultMaxWalkSpeed` (`CharacterMovementComponent.MaxWalkSpeed` _charactermovement)))

(fn `SetMovementSpeedMode`
  (params (NewMovementSpeedMode :type "/Game/CombatSystem/Blueprints/Enums/E_MovementSpeedMode Enum" :default "NewEnumerator0"))
  (if (`|EnumInequality` NewMovementSpeedMode (`self.MovementSpeedMode`))
    (set `self.MovementSpeedMode` (`local.NewMovementSpeedMode`))
    (`/Game/CombatSystem/Blueprints/Components/BP_TargetingComponent.UpdateRotationMode` (`self.TargetingComponent`))))