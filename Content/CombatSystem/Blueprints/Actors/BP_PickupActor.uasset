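; BP_PickupActor is a world item pickup that adds its item to the interacting actor's inventory.
; BeginPlay builds ItemInfo from the data table row set in DataSetup.
; Tick bobs the static mesh by adding a sine-driven Z offset each frame, so its motion depends on frame rate.
; Interact checks for a full inventory, adds the item with zero quantity treated as one, plays a sound and destroys the pickup.
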(event `self.ReceiveBeginPlay`
  (bind _datatableinfo (break `/Game/CombatSystem/Blueprints/Structs/S_ItemSetupData` (`self.DataSetup`)))
  (bind (_datatable _rowname) (break `DataTableRowHandle` _datatableinfo))
  (`/Engine/EditorBlueprintResources/StandardMacros.IsValid` _datatable
    (:`Is Valid`
      (bind _returnvalue (`|GetDataTableRow` _datatable _rowname)
        (:`then`
          (set `self.ItemInfo` (make `/Game/CombatSystem/Blueprints/Structs/S_SlotInfo` _returnvalue _datatableinfo)))))))

(event `self.ReceiveTick`
  (params (DeltaSeconds :type "Float (single-precision)"))
  (`SceneComponent.K2_AddRelativeLocation` (`self.StaticMesh`) (`KismetMathLibrary.MakeVector` 0.0 0.0 (`KismetMathLibrary.Sin` (* (`self.GetGameTimeSinceCreation`) 2.5))) false false))

(event `/Game/CombatSystem/Blueprints/Interfaces/Interactable_BPI.Interact`
  (params (Caller :type "Actor Object Reference"))
  (bind _returnvalue (`self.GetComponentByClass` Caller "/Game/CombatSystem/Blueprints/Components/BP_InventoryComponent.BP_InventoryComponent_C"))
  (bind (_itemstructure _datatableinfo _slotnumber _itemid _quantity) (break `/Game/CombatSystem/Blueprints/Structs/S_SlotInfo` (`self.ItemInfo`)))
  (if (not (`/Game/CombatSystem/Blueprints/Components/BP_InventoryComponent.InventoryFull` _returnvalue))
    (`/Game/CombatSystem/Blueprints/Components/BP_InventoryComponent.AddToInventory` _returnvalue (make `/Game/CombatSystem/Blueprints/Structs/S_SlotInfo` _itemstructure _datatableinfo _slotnumber _itemid (`KismetMathLibrary.SelectInt` 1 _quantity (== _quantity 0))) false false)
    (`GameplayStatics.PlaySoundAtLocation` "/Game/CombatSystem/CourseFiles/SoundFX/SW_PickupItem_Cue.SW_PickupItem_Cue" (`self.K2_GetActorLocation`) (struct) 1.0 1.0 0.0 null null null null)
    (`self.K2_DestroyActor`)))

(fn `UserConstructionScript`)