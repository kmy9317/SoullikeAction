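; Character component that handles incoming point and radial damage for its owner in the combat system.
; Hits end crouching, then go to CombatComponent if blocked, unless unblockable.
; Otherwise it applies stat-mitigated damage through StatsComponent, spawns sparks and sound, and sets Dead at zero.
; Survivors report the damage event and, for melee or knockdown types, enter Disabled with front/back montages chosen by dot product and fetched via PassAnimationMessage.
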(event `self.ReceiveBeginPlay`
  ;[1 0 0] Setup
  (`self.StoreComponents`))

(event `Event Radial Damage`
  (params (DamagedActor :type "Actor Object Reference") (Damage :type "Float (single-precision)") (DamageType :type "DamageType Object Reference") (Origin :type "Vector Structure") (HitInfo :type "HitResult Structure") (InstigatedBy :type "Controller Object Reference") (DamageCauser :type "Actor Object Reference"))
  ;[1 0 0] Damage Triggers
  (`self.StoreDamageInfo` Damage Origin InstigatedBy DamageCauser DamageType)
  (set `self.HitFront?` (`KismetMathLibrary.InRange_FloatFloat` (`Actor.GetDotProductTo` (`self.GetOwner`) (`self.Damage Causer`)) -0.1) :!label _label)
  (bind _biscrouch_ (`self.CheckIsCrouch`))
  (if _biscrouch_
    (`/Game/CombatSystem/Blueprints/Components/BP_MovementComponent.Event ToggleCrouch` (`self.MovementComponent`)))
  (bind _block_success (`self.CanBlockAttack`))
  (if _block_success
    (`/Game/CombatSystem/Blueprints/Components/BP_CombatComponent.Event Block` (`self.CombatComponent`) (`/Game/CombatSystem/Blueprints/DamageType/BP_AttackDamageType.DamageType` (`self.Damage Type`)) (`self.Damage Incoming`) (`self.Damage Causer`) (`self.Hit Location`))
    (else
      (`self.TakeDamage`))))

(event `Event Point Damage`
  (params (DamagedActor :type "Actor Object Reference") (Damage :type "Float (single-precision)") (InstigatedBy :type "Controller Object Reference") (HitLocation :type "Vector Structure") (FHitComponent :type "PrimitiveComponent Object Reference") (BoneName :type Name) (ShotFromDirection :type "Vector Structure") (DamageType :type "DamageType Object Reference") (DamageCauser :type "Actor Object Reference"))
  ;[1 0 0] Damage Triggers
  (`self.StoreDamageInfo` Damage HitLocation InstigatedBy DamageCauser DamageType)
  (goto _label))

(event `TakeDamage`
  (bind _damagetype (`/Game/CombatSystem/Blueprints/DamageType/BP_AttackDamageType.DamageType` (`self.Damage Type`)))
  ;[1 0 0] Damage Triggers
  (`self.ApplyDamage`)
  (`self.ApplyImpactEffect` _damagetype)
  (`self.PlayHitSound` _damagetype)
  (if (!= (`/Game/CombatSystem/Blueprints/Components/BP_StateManagerComponent.GetCurrentState` (`self.StateManagerComponent`)) (struct :`TagName` "Character.State.Dead"))
    (`AISense_Damage.ReportDamageEvent` (`self.GetOwner`) (`Actor.GetOwner` (`self.Damage Causer`)) (`self.Damage Incoming`) (0.0 0.0 0.0) (`self.Hit Location`))
    (`self.CalculateReactAnim` _damagetype)))

(fn `ApplyDamage`
  (locals (L_Damage :type "Float (double-precision)"))
  (bind _statemanagercomponent (`self.StateManagerComponent`))
  (bind _returnvalue (* (`self.Damage Incoming`) (/ (`self.Damage Incoming`) (+ (`self.Damage Incoming`) (`/Game/CombatSystem/Blueprints/Components/BP_StatsComponent.GetCurrentStatValue` (`self.StatsComponent`) "NewEnumerator3")))))
  (set `local.L_Damage` (`KismetMathLibrary.FClamp` _returnvalue 0.0 _returnvalue))
  (`/Game/CombatSystem/Blueprints/Components/BP_StatsComponent.ModifyCurrentStatValue` (`self.StatsComponent`) "NewEnumerator1" (* (`local.L_Damage`) -1.0) false)
  (if (<= (`/Game/CombatSystem/Blueprints/Components/BP_StatsComponent.GetCurrentStatValue` (`self.StatsComponent`) "NewEnumerator1") 0.0)
    (`/Engine/EditorBlueprintResources/StandardMacros.IsValid` _statemanagercomponent
      (:`Is Valid`
        (`/Game/CombatSystem/Blueprints/Components/BP_StateManagerComponent.SetState` _statemanagercomponent (struct :`TagName` "Character.State.Dead"))))))

(fn `ApplyImpactEffect`
  (params (DamageType :type "/Game/CombatSystem/Blueprints/Enums/E_DamageType Enum" :default "NewEnumerator0"))
  (switch `/Game/CombatSystem/Blueprints/Enums/E_DamageType` DamageType
    (:`NewEnumerator0`
      _)
    (:`NewEnumerator1`
      _)
    (:`NewEnumerator2`
      _)
    (:`NewEnumerator3`
      _))
  (`GameplayStatics.SpawnEmitterAtLocation` "/Game/InfinityBladeEffects/Effects/FX_Monsters/FX_Monster_GolemBot/Notifies/P_SparkBurst.P_SparkBurst" (`self.Hit Location`) (struct) (0.7 0.7 0.7)))

(fn `CalculateReactAnim`
  (params (DamageType :type "/Game/CombatSystem/Blueprints/Enums/E_DamageType Enum" :default "NewEnumerator0"))
  (switch `/Game/CombatSystem/Blueprints/Enums/E_DamageType` DamageType
    (:`NewEnumerator1`
      (`self.PerformHitAnim`))
    (:`NewEnumerator2`
      (`self.PerformKnockdown`))))

(fn `CanBlockAttack`
  (returns (`Block Success` :type Boolean))
  (if (`|EnumEquality` (`/Game/CombatSystem/Blueprints/DamageType/BP_AttackDamageType.DamageType` (`self.Damage Type`)) "NewEnumerator3")
    (return false)
    (elif (`/Game/CombatSystem/Blueprints/Components/BP_CombatComponent.bIsBlocking` (`self.CombatComponent`))
      (return true)
      (else
        (return false)))))

(fn `CheckIsCrouch`
  (returns (`bIsCrouch?` :type Boolean))
  (`/Engine/EditorBlueprintResources/StandardMacros.IsValid` (`self.MovementComponent`)
    (:`Is Valid`
      (if (`|EnumEquality` (`/Game/CombatSystem/Blueprints/Components/BP_MovementComponent.GetCurrentSpeedMode` (`self.MovementComponent`)) "NewEnumerator5")
        (return true)
        (else
          (return false))))
    (:`Is Not Valid`
      (return false))))

(fn `ModifyDamageIncoming`
  (params (NewDamage :type "Float (double-precision)"))
  (set `self.Damage Incoming` NewDamage))

(fn `PerformHitAnim`
  (returns (`Success?` :type Boolean))
  (locals (L_HitMonatge :type "AnimMontage Object Reference") (L_HitReactType :type "/Game/CombatSystem/Blueprints/Enums/E_AnimType Enum"))
  (if (`KismetMathLibrary.InRange_FloatFloat` (`Actor.GetDotProductTo` (`self.GetOwner`) (`self.Damage Causer`)) -0.1)
    (set `local.L_HitReactType` "NewEnumerator0")
    (else
      (set `local.L_HitReactType` "NewEnumerator1")))
  (bind _animmontage (message `/Game/CombatSystem/Blueprints/Interfaces/Character_BPI.PassAnimation` (`self.GetOwner`) (`local.L_HitReactType`)))
  (bind _output_get (set `local.L_HitMonatge` _animmontage))
  (`/Engine/EditorBlueprintResources/StandardMacros.IsValid` _output_get
    (:`Is Valid`
      (`/Game/CombatSystem/Blueprints/Components/BP_StateManagerComponent.SetState` (`self.StateManagerComponent`) (struct :`TagName` "Character.State.Disabled"))
      (`Character.PlayAnimMontage` (`self.CharacterRef`) (`local.L_HitMonatge`) 1.0 "None")
      (return true))
    (:`Is Not Valid`
      (return false))))

(fn `PerformKnockdown`
  (returns (`Success?` :type Boolean))
  (locals (L_HitMonatge :type "AnimMontage Object Reference") (L_HitReactType :type "/Game/CombatSystem/Blueprints/Enums/E_AnimType Enum"))
  (if (`KismetMathLibrary.InRange_FloatFloat` (`Actor.GetDotProductTo` (`self.GetOwner`) (`self.Damage Causer`)) -0.1)
    (set `local.L_HitReactType` "NewEnumerator2")
    (else
      (set `local.L_HitReactType` "NewEnumerator3")))
  (bind _animmontage (message `/Game/CombatSystem/Blueprints/Interfaces/Character_BPI.PassAnimation` (`self.GetOwner`) (`local.L_HitReactType`)))
  (bind _output_get (set `local.L_HitMonatge` _animmontage))
  (`/Engine/EditorBlueprintResources/StandardMacros.IsValid` _output_get
    (:`Is Valid`
      (`/Game/CombatSystem/Blueprints/Components/BP_StateManagerComponent.SetState` (`self.StateManagerComponent`) (struct :`TagName` "Character.State.Disabled"))
      (`Character.PlayAnimMontage` (`self.CharacterRef`) (`local.L_HitMonatge`) 1.0 "None")
      (return true))
    (:`Is Not Valid`
      (return false))))

(fn `PlayHitSound`
  (params (DamageType :type "/Game/CombatSystem/Blueprints/Enums/E_DamageType Enum" :default "NewEnumerator0"))
  (`GameplayStatics.PlaySoundAtLocation` (`KismetArrayLibrary.Array_Random` (`|MakeArray` "/Game/CombatSystem/CourseFiles/SoundFX/MeleeHit/SW_MeleeHit_01.SW_MeleeHit_01" "/Game/CombatSystem/CourseFiles/SoundFX/Assassination/SW_MeleeHit_02.SW_MeleeHit_02" "/Game/CombatSystem/CourseFiles/SoundFX/MeleeHit/SW_MeleeHit_03.SW_MeleeHit_03" "/Game/CombatSystem/CourseFiles/SoundFX/MeleeHit/SW_MeleeHit_04.SW_MeleeHit_04" :!type "SoundBase Object Reference")) (`self.Hit Location`) (struct) 1.0 1.0 0.0 null null null null))

(fn `StoreComponents`
  (bind _returnvalue (`self.GetOwner`))
  (add `Actor.OnTakePointDamage` _returnvalue (`|CreateDelegate` :!event `Event Point Damage`))
  (add `Actor.OnTakeRadialDamage` _returnvalue (`|CreateDelegate` :!event `Event Radial Damage`))
  (set `self.EquipmentComponent` (`Actor.GetComponentByClass` _returnvalue "/Game/CombatSystem/Blueprints/Components/BP_EquipmentComponent.BP_EquipmentComponent_C"))
  (set `self.CombatComponent` (`Actor.GetComponentByClass` _returnvalue "/Game/CombatSystem/Blueprints/Components/BP_CombatComponent.BP_CombatComponent_C"))
  (set `self.StatsComponent` (`Actor.GetComponentByClass` _returnvalue "/Game/CombatSystem/Blueprints/Components/BP_StatsComponent.BP_StatsComponent_C"))
  (set `self.StateManagerComponent` (`Actor.GetComponentByClass` _returnvalue "/Game/CombatSystem/Blueprints/Components/BP_StateManagerComponent.BP_StateManagerComponent_C"))
  (set `self.MovementComponent` (`Actor.GetComponentByClass` _returnvalue "/Game/CombatSystem/Blueprints/Components/BP_MovementComponent.BP_MovementComponent_C"))
  (bind _ascharacter (cast `Character` _returnvalue))
  (set `self.CharacterRef` _ascharacter)
  (set `self.CharacterMesh` (`Character.Mesh` _ascharacter))
  (set `self.SkeletalMeshRef` (`SkeletalMeshComponent.GetSkeletalMeshAsset` (`Character.Mesh` (`self.CharacterRef`))))
  (set `self.AnimationSet` (`GameplayStatics.GetObjectClass` (`SkeletalMeshComponent.GetAnimInstance` (`self.CharacterMesh`)))))

(fn `StoreDamageInfo`
  (params (DamageIncoming :type "Float (double-precision)") (HitLocation :type "Vector Structure") (InstigatedBy :type "Controller Object Reference") (DamageCauser :type "Actor Object Reference") (DamageType :type "DamageType Object Reference"))
  (set `self.Damage Incoming` DamageIncoming)
  (set `self.Hit Location` HitLocation)
  (set `self.Instigated By` InstigatedBy)
  (set `self.Damage Causer` DamageCauser)
  (bind _asbp_attack_damage_type (cast `/Game/CombatSystem/Blueprints/DamageType/BP_AttackDamageType` DamageType))
  (set `self.Damage Type` _asbp_attack_damage_type))