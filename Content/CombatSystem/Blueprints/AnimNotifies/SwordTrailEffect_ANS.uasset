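; An anim notify state that shows a weapon trail effect for the duration of its window in an animation.
; On begin it gets the main weapon mesh from the owner through a message call, attaches the trail emitter to it and starts trails between two configurable sockets.
; It hands the spawned component back to the owner, then on end retrieves that stored component and ends its trails.
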(fn `Received_NotifyBegin`
  (params (MeshComp :type "SkeletalMeshComponent Object Reference") (Animation :type "AnimSequenceBase Object Reference") (TotalDuration :type "Float (single-precision)") (EventReference :type "AnimNotifyEventReference Structure (by ref)"))
  (returns (ReturnValue :type Boolean))
  (locals (NewLocalVar :type Boolean))
  (bind _returnvalue (`ActorComponent.GetOwner` MeshComp))
  (bind (_mainweaponmesh _isvalid_) (message `/Game/CombatSystem/Blueprints/Interfaces/Combat_BPI.GetMainWeaponMesh` _returnvalue))
  (if _isvalid_
    (bind _returnvalue_2 (`GameplayStatics.SpawnEmitterAttached` (`self.TrailEffect`) _mainweaponmesh))
    (message `/Game/CombatSystem/Blueprints/Interfaces/Combat_BPI.RefCurrentTrailEffect` _returnvalue _returnvalue_2)
    (`ParticleSystemComponent.BeginTrails` _returnvalue_2 (`self.First Socket Name`) (`self.Second Socket Name`) (`self. Width Mode`) (`self.TrailWidth`))
    (return true)
    (else
      (return false))))

(fn `Received_NotifyEnd`
  (params (MeshComp :type "SkeletalMeshComponent Object Reference") (Animation :type "AnimSequenceBase Object Reference") (EventReference :type "AnimNotifyEventReference Structure (by ref)"))
  (returns (ReturnValue :type Boolean))
  (bind _currenttrail (message `/Game/CombatSystem/Blueprints/Interfaces/Combat_BPI.GetCurrentTrailEffect` (`ActorComponent.GetOwner` MeshComp)))
  (`/Engine/EditorBlueprintResources/StandardMacros.IsValid` _currenttrail
    (:`Is Valid`
      (`ParticleSystemComponent.EndTrails` _currenttrail)
      (return true))
    (:`Is Not Valid`
      (return false))))