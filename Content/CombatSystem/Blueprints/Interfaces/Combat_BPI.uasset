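; Combat_BPI is the Blueprint interface for the combat system, declaring the functions that combat participants implement.
; It covers attack flow and combat resets, tag-driven actions and custom montages, weapon collision, iFrames and damage eligibility.
; It also exposes movement and rotation control, target and assassination queries, health potion updates, and camera, weapon mesh and trail effect access.
; All functions are empty declarations or return defaults, leaving behaviour to implementers.
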(fn `ActivateCollision`
  (params (CollisionPart :type "/Game/CombatSystem/Blueprints/Enums/E_CollisionPart Enum" :default "NewEnumerator0")))

(fn `CanBeAssassinated`
  (returns (True :type Boolean))
  (return false))

(fn `CanReceiveDamage`
  (returns (ReturnValue :type Boolean))
  (return false))

(fn `ContinueAttack`)

(fn `DeactivateCollision`
  (params (CollisionPart :type "/Game/CombatSystem/Blueprints/Enums/E_CollisionPart Enum" :default "NewEnumerator0")))

(fn `GetCurrentTrailEffect`
  (returns (CurrentTrail :type "ParticleSystemComponent Object Reference"))
  (return null))

(fn `GetDesiredRotation`
  (returns (ReturnValue :type "Rotator Structure"))
  (return))

(fn `GetMainWeaponMesh`
  (returns (MainWeaponMesh :type "PrimitiveComponent Object Reference") (`IsValid?` :type Boolean))
  (return null false))

(fn `GetMovementSpeedMode`
  (returns (MovementSpeedMode :type "/Game/CombatSystem/Blueprints/Enums/E_MovementSpeedMode Enum"))
  (return "NewEnumerator0"))

(fn `HasTarget`
  (returns (HasTarget :type Boolean))
  (return false))

(fn `PassCamera`
  (returns (Camera :type "CameraComponent Object Reference") (CameraBoom :type "SpringArmComponent Object Reference"))
  (return null null))

(fn `Perform Action`
  (params (ActionTag :type "GameplayTag Structure") (StateTag :type "GameplayTag Structure" :default (struct :`TagName` "Character.State.GeneralActionState")) (MontageIndex :type Integer) (bRandomIndex :type Boolean))
  (returns (ActionDuration :type "Float (double-precision)") (`bSuccess?` :type Boolean))
  (return 0.0 false))

(fn `PerformAttack`
  (params (AttackType :type "GameplayTag Structure") (AttackIndex :type Integer) (bRandomIndex :type Boolean))
  (returns (AttackDuration :type "Float (double-precision)") (`bSuccess?` :type Boolean))
  (return 0.0 false))

(fn `PerformCustomAction`
  (params (ActionTag :type "GameplayTag Structure") (StateTag :type "GameplayTag Structure") (InMontage :type "AnimMontage Object Reference") (MontagePlayRate :type "Float (double-precision)" :default 1.0) (`bAutoReset?` :type Boolean))
  (returns (`bSuccess?` :type Boolean))
  (return false))

(fn `RefCurrentTrailEffect`
  (params (RefTrailEffectComp :type "ParticleSystemComponent Object Reference"))
  (return))

(fn `ResetAttack`)

(fn `ResetCombat`)

(fn `RotateToTarget`)

(fn `SetCanMove`
  (params (`bCanMove?` :type Boolean)))

(fn `SetiFrames`
  (params (bEnableiFrames :type Boolean)))

(fn `UpdateHealthPotionAmount`
  (params (Amount :type Integer)))

(fn `UpdateMovementMode`
  (params (MovementMode :type "EMovementMode Enum" :default "MOVE_Walking"))
  (returns (Success :type Boolean))
  (return false))