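; BP_SwordAndShield is a weapon actor pairing a main weapon with a shield that has its own mesh and hit collision.
; Equipping and toggling combat attach the shield to the character's hand or stowed socket, and equip state updates the CombatComponent's shield flag.
; Main weapon and shield collisions are switched per part, with shield hits applying point damage.
; Parry effects spawn a block-impact emitter on the shield.
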(event `self.ToggleWeaponCombat`
  (params (`bEnableCombat?` :type Boolean))
  (`parent.ToggleWeaponCombat` `bEnableCombat?`)
  (`self.AttachShield` (select `bool` `bEnableCombat?` :`false` (`self.ShieldAttachSocket`) :`true` (`self.ShieldHandSocket`))))

(event `self.ShieldCollisionComponent.OnHit`
  (params (HitResult :type "HitResult Structure"))
  (bind (_bblockinghit _binitialoverlap _time _distance _location _impactpoint _normal _impactnormal _physmat _hitactor) (`GameplayStatics.BreakHitResult` HitResult))
  (bind _returnvalue (message `/Game/CombatSystem/Blueprints/Interfaces/Combat_BPI.CanReceiveDamage` _hitactor))
  (if _returnvalue
    (`GameplayStatics.ApplyPointDamage` _hitactor (`self.GetDamage`) (`self.GetActorForwardVector` (`self.GetOwner`)) HitResult (`self.GetInstigatorController`) self (`self.Damage Type Class`))))

(event `self.ParryEffects`
  (`GameplayStatics.SpawnEmitterAttached` "/Game/FlexibleCombatSystem/VFX/MeleeVFX/P_BlockImpact.P_BlockImpact" (`self.ShieldMesh`) "ParryVFX"))

(fn `ActivateCollision`
  (params (CollisionPart :type "/Game/CombatSystem/Blueprints/Enums/E_CollisionPart Enum" :default "NewEnumerator0"))
  (switch `/Game/CombatSystem/Blueprints/Enums/E_CollisionPart` CollisionPart
    (:`NewEnumerator0`
      (`/Game/CombatSystem/Blueprints/Components/BP_CollisionComponent.ActivateCollision` (`self.MainWeaponCollisionComponent`)))
    (:`NewEnumerator3`
      (`/Game/CombatSystem/Blueprints/Components/BP_CollisionComponent.ActivateCollision` (`self.ShieldCollisionComponent`)))))

(fn `AttachShield`
  (params (AttachSocket :type Name))
  (`SceneComponent.K2_AttachToComponent` (`self.ShieldMesh`) (`Character.Mesh` (cast `Character` (`self.GetOwner`) :!pure true)) AttachSocket "KeepRelative" "KeepRelative" "KeepRelative" true))

(fn `DeactivateCollision`
  (params (CollisionPart :type "/Game/CombatSystem/Blueprints/Enums/E_CollisionPart Enum" :default "NewEnumerator0"))
  (switch `/Game/CombatSystem/Blueprints/Enums/E_CollisionPart` CollisionPart
    (:`NewEnumerator0`
      (`/Game/CombatSystem/Blueprints/Components/BP_CollisionComponent.DeactivateCollision` (`self.MainWeaponCollisionComponent`)))
    (:`NewEnumerator3`
      (`/Game/CombatSystem/Blueprints/Components/BP_CollisionComponent.DeactivateCollision` (`self.ShieldCollisionComponent`)))))

(fn `GetSubWeaponMesh`
  (returns (SubWeaponMesh :type "PrimitiveComponent Object Reference"))
  (bind _shieldmesh (`self.ShieldMesh`))
  (`/Engine/EditorBlueprintResources/StandardMacros.IsValid` _shieldmesh
    (:`Is Valid`
      (return _shieldmesh))
    (:`Is Not Valid`
      (return null))))

(fn `OnEquipped`
  (`parent.OnEquipped`)
  (`self.AttachShield` (select `bool` (`/Game/CombatSystem/Blueprints/Components/BP_CombatComponent.IsCombatEnabled?` (`self.CombatComponent`)) :`false` (`self.ShieldAttachSocket`) :`true` (`self.ShieldHandSocket`)))
  (`/Game/CombatSystem/Blueprints/Components/BP_CollisionComponent.SetCollisionMesh` (`self.ShieldCollisionComponent`) (`self.ShieldMesh`))
  (`/Game/CombatSystem/Blueprints/Components/BP_CollisionComponent.AddActorToIgnore` (`self.ShieldCollisionComponent`) (`self.GetOwner`))
  (`/Game/CombatSystem/Blueprints/Components/BP_CombatComponent.SetShieldEquipped` (`self.CombatComponent`) true))

(fn `OnUnequipped`
  (`parent.OnUnequipped`)
  (`/Game/CombatSystem/Blueprints/Components/BP_CombatComponent.SetShieldEquipped` (`self.CombatComponent`) false))

(fn `UserConstructionScript`
  (`parent.UserConstructionScript`))