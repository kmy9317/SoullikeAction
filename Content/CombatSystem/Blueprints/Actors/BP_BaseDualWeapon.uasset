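; Base dual-wield weapon actor that extends its parent weapon with an off-hand mesh and extra hit detection for that weapon and the owner's right foot.
; The off-hand mesh snaps to a hand or stowed socket on the character as combat toggles or on equip.
; Collision components switch on and off per body part, ignore the owner, and apply point damage to hit actors that can receive damage.
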(event `self.ToggleWeaponCombat`
  (params (`bEnableCombat?` :type Boolean))
  (`parent.ToggleWeaponCombat` `bEnableCombat?`)
  (`self.AttachOff-HandWeapon` (select `bool` `bEnableCombat?` :`false` (`self.SecondWeaponAttachSocket`) :`true` (`self.SecondWeaponHandSocket`))))

(event `self.Off-handWeaponCollisionComponent.OnHit`
  (params (HitResult :type "HitResult Structure"))
  (bind (_bblockinghit _binitialoverlap _time _distance _location _impactpoint _normal _impactnormal _physmat _hitactor) (`GameplayStatics.BreakHitResult` HitResult))
  (bind _returnvalue (message `/Game/CombatSystem/Blueprints/Interfaces/Combat_BPI.CanReceiveDamage` _hitactor))
  (if _returnvalue
    (`GameplayStatics.ApplyPointDamage` _hitactor (`self.GetDamage`) (`self.GetActorForwardVector` (`self.GetOwner`)) HitResult (`self.GetInstigatorController`) self (`self.Damage Type Class`))))

(event `self.BP_RightFoot.OnHit`
  (params (HitResult :type "HitResult Structure"))
  (bind (_bblockinghit _binitialoverlap _time _distance _location _impactpoint _normal _impactnormal _physmat _hitactor) (`GameplayStatics.BreakHitResult` HitResult))
  (bind _returnvalue (message `/Game/CombatSystem/Blueprints/Interfaces/Combat_BPI.CanReceiveDamage` _hitactor))
  (if _returnvalue
    (`GameplayStatics.ApplyPointDamage` _hitactor (`self.GetDamage`) (`self.GetActorForwardVector` (`self.GetOwner`)) HitResult (`self.GetInstigatorController`) self (`self.Damage Type Class`))))

(fn `ActivateCollision`
  (params (CollisionPart :type "/Game/CombatSystem/Blueprints/Enums/E_CollisionPart Enum" :default "NewEnumerator0"))
  (switch `/Game/CombatSystem/Blueprints/Enums/E_CollisionPart` CollisionPart
    (:`NewEnumerator0`
      (`/Game/CombatSystem/Blueprints/Components/BP_CollisionComponent.ActivateCollision` (`self.MainWeaponCollisionComponent`)))
    (:`NewEnumerator1`
      (`/Game/CombatSystem/Blueprints/Components/BP_CollisionComponent.ActivateCollision` (`self.Off-handWeaponCollisionComponent`)))
    (:`NewEnumerator2`
      (`/Game/CombatSystem/Blueprints/Components/BP_CollisionComponent.ActivateCollision` (`self.BP_RightFoot`)))))

(fn `AttachOff-HandWeapon`
  (params (Socket :type Name))
  (`SceneComponent.K2_AttachToComponent` (`self.Off-handWeaponMesh`) (`Character.Mesh` (cast `Character` (`self.GetOwner`) :!pure true)) Socket "SnapToTarget" "SnapToTarget" "SnapToTarget" true))

(fn `DeactivateCollision`
  (params (CollisionPart :type "/Game/CombatSystem/Blueprints/Enums/E_CollisionPart Enum" :default "NewEnumerator0"))
  (switch `/Game/CombatSystem/Blueprints/Enums/E_CollisionPart` CollisionPart
    (:`NewEnumerator0`
      (`/Game/CombatSystem/Blueprints/Components/BP_CollisionComponent.DeactivateCollision` (`self.MainWeaponCollisionComponent`)))
    (:`NewEnumerator1`
      (`/Game/CombatSystem/Blueprints/Components/BP_CollisionComponent.DeactivateCollision` (`self.Off-handWeaponCollisionComponent`)))
    (:`NewEnumerator2`
      (`/Game/CombatSystem/Blueprints/Components/BP_CollisionComponent.DeactivateCollision` (`self.BP_RightFoot`)))))

(fn `OnEquipped`
  (`parent.OnEquipped`)
  (`/Game/CombatSystem/Blueprints/Components/BP_CollisionComponent.SetCollisionMesh` (`self.Off-handWeaponCollisionComponent`) (`self.Off-handWeaponMesh`))
  (`/Game/CombatSystem/Blueprints/Components/BP_CollisionComponent.SetCollisionMesh` (`self.BP_RightFoot`) (`Character.Mesh` (cast `Character` (`self.GetOwner`) :!pure true)))
  (`self.AttachOff-HandWeapon` (select `bool` (`/Game/CombatSystem/Blueprints/Components/BP_CombatComponent.IsCombatEnabled?` (`self.CombatComponent`)) :`false` (`self.SecondWeaponAttachSocket`) :`true` (`self.SecondWeaponHandSocket`)))
  (`/Game/CombatSystem/Blueprints/Components/BP_CollisionComponent.AddActorToIgnore` (`self.Off-handWeaponCollisionComponent`) (`self.GetOwner`))
  (`/Game/CombatSystem/Blueprints/Components/BP_CollisionComponent.AddActorToIgnore` (`self.BP_RightFoot`) (`self.GetOwner`)))

(fn `UserConstructionScript`
  (`parent.UserConstructionScript`))