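; Base shield equipment actor for the combat system, registering itself as the owner's shield weapon while equipped.
; On equip it sets its equipped state, attaches to the hand or stowed socket depending on combat mode, binds to combat toggling and readies weapon collision, ignoring the owner.
; Action montages are selected by gameplay tag for attacks, dodging, blocking and combat transitions.
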(fn `Get Action Montages`
  (params (CharacterAction :type "GameplayTag Structure"))
  (returns (Montages :type "Array of AnimMontage Object Reference"))
  (`|SwitchGameplayTag` CharacterAction
    (:`Character.Action.Attack.LightAttack`
      (return (`self.LightAttackMontage`)))
    (:`Character.Action.Attack.HeavyAttack`
      (return (`self.HeavyAttackMontages`)))
    (:`Character.Action.Attack.ChargeAttack`
      (return (`self.ChargeAttackMontages`)))
    (:`Character.Action.Attack.SprintAttack`
      (return (`self.SprintAttackMontages`)))
    (:`Character.Action.Attack.FallingAttack`
      (return (`self.FallingAttackMontages`)))
    (:`Character.Action.Dodge`
      (return (`self.DodgeMontage`)))
    (:`Character.Action.EnterCombat`
      (return (`|MakeArray` (`self.EnterCombat`))))
    (:`Character.Action.ExitCombat`
      (return (`|MakeArray` (`self.ExitCombat`))))
    (:`Character.Action.BlockAttack`
      (return (`self.BlockAnimations`)))))

(fn `OnEquipped`
  (`self.SetIsEquipped` true)
  (`self.AttachActor` (`self.AttachSocketName`))
  (`/Game/CombatSystem/Blueprints/Components/BP_StateManagerComponent.SetState` (`self.BP_StateManagerComponent`) (struct :`TagName` "Weapon.State.Equipped"))
  (bind _output_get (set `self.CombatComponent` (`self.GetComponentByClass` (`self.GetOwner`) "/Game/CombatSystem/Blueprints/Components/BP_CombatComponent.BP_CombatComponent_C")))
  (add `/Game/CombatSystem/Blueprints/Components/BP_CombatComponent.OnCombatToggled` _output_get (`|CreateDelegate` :!event `ToggleWeaponCombat`))
  (set `self.OwnerStateManager` (`self.GetComponentByClass` (`self.GetOwner`) "/Game/CombatSystem/Blueprints/Components/BP_StateManagerComponent.BP_StateManagerComponent_C"))
  (`self.AttachActor` (select `bool` (`/Game/CombatSystem/Blueprints/Components/BP_CombatComponent.IsCombatEnabled?` (`self.CombatComponent`)) :`false` (`self.AttachSocketName`) :`true` (`self.HandSocketName`)))
  (`/Game/CombatSystem/Blueprints/Components/BP_CombatComponent.SetShieldWeapon` (`self.CombatComponent`) self)
  (`/Game/CombatSystem/Blueprints/Components/BP_CollisionComponent.SetCollisionMesh` (`self.MainWeaponCollisionComponent`) (`self.GetItemMesh`))
  (`/Game/CombatSystem/Blueprints/Components/BP_CollisionComponent.AddActorToIgnore` (`self.MainWeaponCollisionComponent`) (`self.GetOwner`)))

(fn `OnUnequipped`
  (`parent.OnUnequipped`)
  (`/Game/CombatSystem/Blueprints/Components/BP_CombatComponent.SetShieldWeapon` (`self.CombatComponent`) null))

(fn `UserConstructionScript`
  (`parent.UserConstructionScript`))