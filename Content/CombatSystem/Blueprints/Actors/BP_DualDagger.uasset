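; BP_DualDagger is a dual dagger weapon actor in the combat system, with an offhand weapon mesh for the second blade.
; Its GetSubWeaponMesh function returns that offhand mesh when it is valid, and nothing otherwise.
; The event graph holds only disabled default events, and the construction script just calls its parent, so the Blueprint adds no other logic.
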(fn `GetSubWeaponMesh`
  (returns (SubWeaponMesh :type "PrimitiveComponent Object Reference"))
  (bind _off_handweaponmesh (`self.Off-handWeaponMesh`))
  (`/Engine/EditorBlueprintResources/StandardMacros.IsValid` _off_handweaponmesh
    (:`Is Valid`
      (return _off_handweaponmesh))
    (:`Is Not Valid`
      (return null))))

(fn `UserConstructionScript`
  (`parent.UserConstructionScript`))