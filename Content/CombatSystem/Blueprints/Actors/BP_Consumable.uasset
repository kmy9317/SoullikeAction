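; BP_Consumable is a limited-use item actor, apparently a health potion or similar, that modifies one of its owner's stats.
; Uses reset to maximum on BeginPlay, and PerformItemAction, while any remain, asks the owner via interface message to play the UseItem montage action.
; A separate ConsumeItem event decrements the count, sends it to the owner as the health potion amount and modifies the configured stat through BP_StatsComponent.
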(event `self.ReceiveBeginPlay`
  (`parent.ReceiveBeginPlay`)
  (set `self.CurrentNumberOfUses` (`self.MaxNumberOfUses`)))

(event `self.PerformItemAction`
  (if (> (`self.CurrentNumberOfUses`) 0)
    (bind _bsuccess_ (message `/Game/CombatSystem/Blueprints/Interfaces/Combat_BPI.PerformCustomAction` (`self.GetOwner`) (struct :`TagName` "Character.Action.UseItem") (struct :`TagName` "Character.State.GeneralActionState") (`self.UseItemMontage`) 1.0 false))
    (if _bsuccess_
      _)))

(event `ConsumeItem`
  (bind _result (`/Engine/EditorBlueprintResources/StandardMacros.DecrementInt` (`self.CurrentNumberOfUses`))
    (:`  `
      (message `/Game/CombatSystem/Blueprints/Interfaces/Combat_BPI.UpdateHealthPotionAmount` (`self.GetOwner`) _result)
      (`/Game/CombatSystem/Blueprints/Components/BP_StatsComponent.ModifyCurrentStatValue` (`self.GetComponentByClass` (`self.GetOwner`) "/Game/CombatSystem/Blueprints/Components/BP_StatsComponent.BP_StatsComponent_C") (`self.Stat`) (`self.ModificationValue`) (`self.Should Regenerate?`)))))

(fn `UserConstructionScript`
  (`parent.UserConstructionScript`))