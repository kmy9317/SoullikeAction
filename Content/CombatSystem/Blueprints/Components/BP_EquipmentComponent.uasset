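; Character equipment component that spawns, tracks and destroys equipped item actors, starting from a default loadout.
; EquipItem replaces same-class items and adds Main Hand items to inventory, while tag queries find equipped items or trigger their actions.
; Equip/unequip events handle only Main Hand, swapping the weapon actor from item data or removing it and disabling combat.
; StatsComponent is cached but unused, despite the events' stat-related names.
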(event `EquipItemAddStats`
  (params (ItemType :type "/Game/CombatSystem/Blueprints/Enums/E_ItemType Enum" :default "NewEnumerator3") (ItemInfo :type "/Game/CombatSystem/Blueprints/Structs/S_SlotInfo Structure"))
  (set `self.ItemInfo` ItemInfo)
  (`self.AddEquipment` ItemType))

(event `UnequipItemRemoveStats`
  (params (ItemType :type "/Game/CombatSystem/Blueprints/Enums/E_ItemType Enum" :default "NewEnumerator3"))
  (`self.DeleteEquipment` ItemType))

(fn `AddEquipment`
  (params (ItemType :type "/Game/CombatSystem/Blueprints/Enums/E_ItemType Enum" :default "NewEnumerator3"))
  (if (== (`.Quantity_14_EE71000140EF6615DBB22FAA646B9555` (break `/Game/CombatSystem/Blueprints/Structs/S_SlotInfo` (select `/Game/CombatSystem/Blueprints/Enums/E_ItemType` ItemType :`NewEnumerator12` (`self.MainHandInfo`)))) 0)
    _
    (else
      _))
  (switch `/Game/CombatSystem/Blueprints/Enums/E_ItemType` (`local.ItemType`)
    (:`NewEnumerator12`
      (`self.ReplaceWeaponActor` (`local.ItemType`)))))

(fn `DeleteEquipment`
  (params (ItemType :type "/Game/CombatSystem/Blueprints/Enums/E_ItemType Enum" :default "NewEnumerator3"))
  (switch `/Game/CombatSystem/Blueprints/Enums/E_ItemType` ItemType
    (:`NewEnumerator12`
      (bind _currentweapon (message `/Game/CombatSystem/Blueprints/Interfaces/Character_BPI.PassMainWeapon` (`self.CharacterRef`)))
      (`/Engine/EditorBlueprintResources/StandardMacros.IsValid` _currentweapon
        (:`Is Valid`
          (`KismetArrayLibrary.Array_RemoveItem` (`self.EquippedItems`) _currentweapon)
          (`self.UnequipItem` _currentweapon)
          (set `self.MainHandInfo` (struct))
          (`/Game/CombatSystem/Blueprints/Components/BP_CombatComponent.Set Combat Enabled` (`self.CombatComponent`) false))))))

(fn `EquipItem`
  (params (InEquipment :type "/Game/CombatSystem/Blueprints/Actors/BP_BaseEquippable Class Reference"))
  (returns (`bSuccess?` :type Boolean))
  (bind _returnvalue (`self.GetOwner`))
  (bind _aspawn (cast `Pawn` _returnvalue :!pure true))
  (if (`KismetSystemLibrary.IsValidClass` InEquipment)
    (`|ExecutionSequence`
      (:`then_0`
        (for _array_element (`self.EquippedItems`)
          (if (== (`GameplayStatics.GetObjectClass` _array_element) (`local.InEquipment`))
            (`self.UnequipItem` _array_element))))
      (:`then_1`
        (bind _returnvalue_2 (`|SpawnActorFromClass` (`local.InEquipment`) (`Actor.GetTransform` _returnvalue) "Undefined" "OverrideRootScale" _aspawn (struct) _aspawn))
        (`/Game/CombatSystem/Blueprints/Actors/BP_BaseEquippable.OnEquipped` _returnvalue_2)
        (`KismetArrayLibrary.Array_AddUnique` (`self.EquippedItems`) _returnvalue_2)
        (switch `/Game/CombatSystem/Blueprints/Enums/E_ItemType` (`/Game/CombatSystem/Blueprints/Actors/BP_BaseEquippable.ItemType` _returnvalue_2)
          (:`NewEnumerator3`
            (return true))
          (:`NewEnumerator12`
            (`/Game/CombatSystem/Blueprints/Actors/BP_BaseEquippable.AddToInventory` _returnvalue_2 (`self.CharacterRef`))
            (return true)))))
    (else
      (return false))))

(fn `GetEquippedItembyTag`
  (params (ItemTag :type "GameplayTag Structure"))
  (returns (ReturnValue :type "/Game/CombatSystem/Blueprints/Actors/BP_BaseEquippable Object Reference"))
  (for _array_element (`self.EquippedItems`)
    (`/Engine/EditorBlueprintResources/StandardMacros.IsValid` _array_element
      (:`Is Valid`
        (bind _returnvalue (`/Game/CombatSystem/Blueprints/Actors/BP_BaseEquippable.HasMatchingGameplayTag` _array_element (`local.ItemTag`) false))
        (if _returnvalue
          (return _array_element)))))
  (return null))

(fn `InitializeEquipment`
  (`self.StoreComponents`)
  (`|ExecutionSequence`
    (:`then_0`
      (for _array_element (`self.EquippedItems`)
        (`self.UnequipItem` _array_element)))
    (:`then_1`
      (for _array_element_2 (`self.StartingEquipment`)
        (if (`KismetSystemLibrary.IsValidClass` _array_element_2)
          (`self.EquipItem` _array_element_2))))))

(fn `PerformActionFromItem`
  (params (ItemTag :type "GameplayTag Structure"))
  (returns (`Success?` :type Boolean))
  (for _array_element (`self.EquippedItems`)
    (`/Engine/EditorBlueprintResources/StandardMacros.IsValid` _array_element
      (:`Is Valid`
        (bind _returnvalue (`/Game/CombatSystem/Blueprints/Actors/BP_BaseEquippable.HasMatchingGameplayTag` _array_element (`local.ItemTag`) false))
        (if _returnvalue
          (`/Game/CombatSystem/Blueprints/Actors/BP_BaseEquippable.PerformItemAction` _array_element)
          (return true)))))
  (return false))

(fn `ReplaceWeaponActor`
  (params (ItemType :type "/Game/CombatSystem/Blueprints/Enums/E_ItemType Enum" :default "NewEnumerator3"))
  (bind _characterref (`self.CharacterRef`))
  (bind (_itemstructure _datatableinfo) (break `/Game/CombatSystem/Blueprints/Structs/S_SlotInfo` (`self.ItemInfo`)))
  (switch `/Game/CombatSystem/Blueprints/Enums/E_ItemType` ItemType
    (:`NewEnumerator12`
      (bind _returnvalue (`|SpawnActorFromClass` (`.ItemClass_33_4623D10E43AE23D45FB063818D1CFEE5` (break `/Game/CombatSystem/Blueprints/Structs/S_ItemData` _itemstructure)) (`Actor.GetTransform` _characterref) "Undefined" "OverrideRootScale" _characterref (make `/Game/CombatSystem/Blueprints/Structs/S_ItemSetupData` _datatableinfo) _characterref))
      (set `self.MainHandInfo` (`self.ItemInfo`))
      (bind _currentweapon (message `/Game/CombatSystem/Blueprints/Interfaces/Character_BPI.PassMainWeapon` (`self.CharacterRef`)))
      (`/Engine/EditorBlueprintResources/StandardMacros.IsValid` _currentweapon
        (:`Is Valid`
          (`KismetArrayLibrary.Array_RemoveItem` (`self.EquippedItems`) _currentweapon)
          (`self.UnequipItem` _currentweapon))
        (:`Is Not Valid`
          _))
      (`/Game/CombatSystem/Blueprints/Actors/BP_BaseEquippable.OnEquipped` _returnvalue)
      (`KismetArrayLibrary.Array_AddUnique` (`self.EquippedItems`) _returnvalue))))

(fn `StoreComponents`
  (bind _returnvalue (`self.GetOwner`))
  (bind _ascharacter (cast `Character` _returnvalue))
  (set `self.CharacterRef` _ascharacter)
  (set `self.InventoryComponent` (`Actor.GetComponentByClass` _returnvalue "/Game/CombatSystem/Blueprints/Components/BP_InventoryComponent.BP_InventoryComponent_C"))
  (set `self.StatsComponent` (`Actor.GetComponentByClass` _returnvalue "/Game/CombatSystem/Blueprints/Components/BP_StatsComponent.BP_StatsComponent_C"))
  (set `self.CombatComponent` (`Actor.GetComponentByClass` _returnvalue "/Game/CombatSystem/Blueprints/Components/BP_CombatComponent.BP_CombatComponent_C")))

(fn `UnequipItem`
  (params (`Equipment to Unequip` :type "/Game/CombatSystem/Blueprints/Actors/BP_BaseEquippable Object Reference"))
  (`/Engine/EditorBlueprintResources/StandardMacros.IsValid` `Equipment to Unequip`
    (:`Is Valid`
      (`/Game/CombatSystem/Blueprints/Actors/BP_BaseEquippable.OnUnequipped` `Equipment to Unequip`)
      (`Actor.K2_DestroyActor` (`local.Equipment to Unequip`)))))