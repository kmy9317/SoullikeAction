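; BP_SkeletonEnemy is a skeleton enemy Blueprint in the combat system's AI, with almost no logic of its own.
; It exposes its WeaponMesh through two getters: GetWeaponMesh returns it directly, while GetMainWeaponMesh adds a validity check and flag.
; The event graph holds only disabled placeholder events, and the construction script just calls the parent.
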(fn `GetMainWeaponMesh`
  (returns (MainWeaponMesh :type "PrimitiveComponent Object Reference") (`IsValid?` :type Boolean))
  (bind _weaponmesh (`self.WeaponMesh`))
  (`/Engine/EditorBlueprintResources/StandardMacros.IsValid` _weaponmesh
    (:`Is Valid`
      (return _weaponmesh true))
    (:`Is Not Valid`
      (return null false))))

(fn `GetWeaponMesh`
  (returns (ReturnValue :type "PrimitiveComponent Object Reference"))
  (return (`self.WeaponMesh`)))

(fn `UserConstructionScript`
  (`parent.UserConstructionScript`))